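; Player character Blueprint for cursor-driven, mouse-wheel control that keeps the cursor visible and yaws the pawn toward it every tick.
; Scrolling down click-moves to the cursor's world point via SimpleMoveToLocation; scrolling up runs a placeholder attack that prints the hovered object's name behind a DoOnce and Delay cooldown.
; Axis movement and turning inputs gated by TestMovement are temporary test controls.
; SwitchPlayingCue only sets the IsPlayingCue flag.
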(event Custom|Switch%20Playing%20Cue
  (params (NewValue :type Boolean))
  ;[1 1 1] Switches audio cue
  (Variables|Default|SetbIsPlayingCue NewValue))

(event EventTick
  (params (DeltaSeconds :type Float%20%28single-precision%29))
  ;[1 1 1] Rotates the pawn to always look at the cursor
  (Transformation|SetActorRotation (Math|Rotator|MakeRotator 0.0 0.0 (.Yaw (Math|Rotator|BreakRotator (Math|Rotator|FindLookatRotation (Transformation|GetActorLocation) (Utilities|CursortoWorld)))))))

(event EventBeginPlay
  ;[1 1 1] Ensures mouse can always be seen
  (Variables|/Script/Engine.PlayerController|SetbShowMouseCursor (Game|GetPlayerController 0) true))

(event Input|AxisEvents|InputAxisinputTest_Forward
  (params (AxisValue :type Float%20%28single-precision%29))
  ;[1 0 0] All for testing purposes until "follow mouse" movement is implemented
  (if (Variables|Default|GettestMovement)
    (Pawn|Input|AddMovementInput (Math|Vector|GetForwardVector (Math|Rotator|MakeRotator 0.0 0.0 (.Yaw (Math|Rotator|BreakRotator (Pawn|GetControlRotation :!class /Script/Engine.Pawn))))) AxisValue false)))

(event Input|AxisEvents|InputAxisinputTest_Right
  (params (AxisValue :type Float%20%28single-precision%29))
  ;[1 0 0] All for testing purposes until "follow mouse" movement is implemented
  (if (Variables|Default|GettestMovement)
    (Pawn|Input|AddMovementInput (Math|Vector|GetRightVector (Math|Rotator|MakeRotator 0.0 0.0 (.Yaw (Math|Rotator|BreakRotator (Pawn|GetControlRotation :!class /Script/Engine.Pawn))))) AxisValue false)))

(event Input|AxisEvents|InputAxisinput_MouseWheel
  (params (AxisValue :type Float%20%28single-precision%29))
  (bind _attackcooldowntimer (Variables|Default|GetattackCooldownTimer))
  ;[1 1 1] Detects when the mouse-wheel is being scrolled, and what direction
  (if (< 0.0 AxisValue)
    (Development|PrintString "Scrolled Up" true false "(R=0.000000,G=0.660000,B=1.000000,A=1.000000)" 1.0)
    ;[1 1 1] Scroll up - Break Things
    (Utilities|FlowControl|DoOnce (Variables|Default|GetattackCooldown) :!label _label
      (:Completed
        (Development|PrintString (Utilities|GetObjectName (Utilities|CursortoObject)) true false "(R=0.000000,G=0.660000,B=1.000000,A=1.000000)" _attackcooldowntimer)
        (Utilities|FlowControl|Delay _attackcooldowntimer)
        (goto _label Reset)))
    (elif (> 0.0 AxisValue)
      (Development|PrintString "Scrolled Down" true false "(R=0.000000,G=0.660000,B=1.000000,A=1.000000)" 1.0)
      ;[1 1 1] Scroll down - Move and Interact
      (AI|Navigation|SimpleMovetoLocation (Game|GetPlayerController 0) (Utilities|CursortoWorld)))))

(event Input|AxisEvents|InputAxisinputTest_Turn
  (params (AxisValue :type Float%20%28single-precision%29))
  ;[1 0 0] All for testing purposes until "follow mouse" movement is implemented
  (if (Variables|Default|GettestMovement)
    (Pawn|Input|AddControllerYawInput AxisValue)))

(fn ConstructionScript)