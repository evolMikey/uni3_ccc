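; bp_AudioCue is a trigger actor that plays a sound cue when a player character enters its TriggerZone.
; On overlap, it skips characters already playing a cue, otherwise sets that character's playing flag and plays AudioEffect at its location.
; The flag clears after the sound's duration plus a short delay, preventing overlapping cues per character.
; It also stores the player index in IController, which this graph never reads.
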(event OnActorBeginOverlap(TriggerZone)
  (params (OverlappedActor :type Actor%20Object%20Reference) (OtherActor :type Actor%20Object%20Reference))
  (bind _audioeffect (Variables|Default|GetAudioEffect))
  (bind _asbp_player_char (Utilities|Casting|CastTobp_PlayerChar OtherActor))
  (if (not (Variables|/Game/Character/bp_PlayerChar.bp_PlayerChar_C|GetbIsPlayingCue _asbp_player_char))
    (bind _playerindex (Class|TurnBasedBlueprintLibrary|GetMyPlayerIndex _asbp_player_char))
    (Variables|Default|SetiController _playerindex)
    (Default|SwitchPlayingCue _asbp_player_char true)
    (Audio|PlaySoundatLocation OtherActor _audioeffect (Transformation|GetActorLocation OtherActor))
    (Utilities|FlowControl|Delay (+ (Variables|/Script/Engine.SoundBase|GetDuration _audioeffect) 1.0))
    (Default|SwitchPlayingCue _asbp_player_char false)))

(fn ConstructionScript)